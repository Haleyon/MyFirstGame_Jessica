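; Lamp post prop with two rect lights whose on/off state follows the IsLightOn flag.
; The construction script sets both lights to LightIntensity, or zeroes and hides them when off.
; ToggleLamp reassigns the flag to itself without inverting it, then applies intensity, hiding the two light-part components instead when off.
; Neither path restores visibility when on, and the stock events are unused.
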(event `ToggleLamp`
  (bind _output_get (set `self.IsLightOn` (`self.IsLightOn`)))
  (if _output_get
    (`LightComponent.SetIntensity` (`self.RectLight1`) (`self.LightIntensity`))
    (`LightComponent.SetIntensity` (`self.RectLight`) (`self.LightIntensity`))
    (else
      (`LightComponent.SetIntensity` (`self.RectLight`) 0.0)
      (`LightComponent.SetIntensity` (`self.RectLight1`) 0.0)
      (`SceneComponent.SetVisibility` (`self.SM_LampPost_LightPart02`) false false)
      (`SceneComponent.SetVisibility` (`self.SM_LampPost_LightPart01`) false false))))

(fn `UserConstructionScript`
  (bind _rectlight1 (`self.RectLight1`))
  (if (`self.IsLightOn`)
    (`LightComponent.SetIntensity` _rectlight1 (`self.LightIntensity`))
    (`LightComponent.SetIntensity` (`self.RectLight`) (`self.LightIntensity`))
    (else
      (`LightComponent.SetIntensity` _rectlight1 0.0)
      (`LightComponent.SetIntensity` (`self.RectLight`) 0.0)
      (`SceneComponent.SetVisibility` (`self.RectLight`) false false)
      (`SceneComponent.SetVisibility` _rectlight1 false false))))