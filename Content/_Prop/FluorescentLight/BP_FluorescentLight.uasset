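; Fluorescent light prop Blueprint with a lamp that can be switched on or off.
; ToggleLamp stores the IsLightOn state and sets the lamp light to LightIntensity or zero.
; The construction script applies the same state from IsLightOn, so the editor reflects it.
; In both graphs only the off branch changes mesh visibility, hiding one light mesh; turning on does not show it again.
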(event `self.ReceiveBeginPlay`)

(event `ToggleLamp`
  (params (IsOn :type Boolean))
  (bind _lamplight (`self.LampLight`))
  (bind _output_get (set `self.bIsLightOn` IsOn))
  (if _output_get
    (`LightComponent.SetIntensity` _lamplight (`self.LightIntensity`))
    (else
      (`LightComponent.SetIntensity` _lamplight 0.0)
      (`SceneComponent.SetVisibility` (`self.SM_FluorescentLight_SM_FluorescentLight_LOD1_001`) _output_get false))))

(fn `UserConstructionScript`
  (bind _lamplight (`self.LampLight`))
  (if (`self.bIsLightOn`)
    (`LightComponent.SetIntensity` _lamplight (`self.LightIntensity`))
    (else
      (`LightComponent.SetIntensity` _lamplight 0.0)
      (`SceneComponent.SetVisibility` (`self.SM_FluorescentLight_SM_FluorescentLight_LOD1_001`) false false))))